(event `self.ReceiveBeginPlay`
  ;[1 1 1] Connecting the Health bar Interface to the player
  (bind _returnvalue (`|CreateWidget` "/Game/Blueprints/UI/WB_HealthBar.WB_HealthBar_C" (`GameplayStatics.GetPlayerController` 0)))
  (bind _output_get (set `self.WB_MainInterface` _returnvalue))
  (`UserWidget.AddToViewport` _output_get 0)
  (bind _output_get_2 (set `self.CurrentHealth` (`self.MaxHealth`)))
  (`/Game/Blueprints/UI/WB_HealthBar.UpdateHealthBar` (`self.WB_MainInterface`) _output_get_2 (`self.MaxHealth`))
  ;[1 1 1] Connect to Back to Hub Button
  (bind _returnvalue_2 (`|CreateWidget` "/Game/Blueprints/UI/WB_BackToHubBtn.WB_BackToHubBtn_C" (`GameplayStatics.GetPlayerController` 0)))
  (bind _output_get_3 (set `self.WB_BackToHabBtn` _returnvalue_2))
  (`UserWidget.AddToViewport` _output_get_3 0)
  ;[1 1 1] Connect To List of Tasks
  (bind _returnvalue_3 (`|CreateWidget` "/Game/Blueprints/UI/WB_ListOfTasks.WB_ListOfTasks_C" (`GameplayStatics.GetPlayerController` 0)))
  (`UserWidget.AddToViewport` _returnvalue_3 0)
  (bind _returnvalue_4 (`|CreateWidget` "/Game/Blueprints/UI/WB_ImplantStore.WB_ImplantStore_C" (`GameplayStatics.GetPlayerController` 0)))
  (bind _output_get_4 (set `self.WB_ImplantStore` _returnvalue_4))
  (`UserWidget.AddToViewport` _output_get_4 0)
  (`Widget.SetVisibility` _output_get_4 "Hidden"))

(event `Key|I`
  (params (Key :type "Key Structure"))
  (bind _returnvalue (`GameplayStatics.GetPlayerController` 0))
  (bind _wb_implantstore (`self.WB_ImplantStore`))
  (:`Pressed`
    (`/Engine/EditorBlueprintResources/StandardMacros.FlipFlop`
      (:`A`
        (set `Widget.Visibility` "SelfHitTestInvisible" _wb_implantstore)
        (set `PlayerController.bShowMouseCursor` true _returnvalue))
      (:`B`
        (set `Widget.Visibility` "Hidden" _wb_implantstore)
        (set `PlayerController.bShowMouseCursor` false _returnvalue)
        (`/Game/Blueprints/UI/WB_ImplantStore.CleanUpSelect` (`self.WB_ImplantStore`))))))

(event `self.ReceiveAnyDamage`
  (params (Damage :type "Float (single-precision)") (DamageType :type "DamageType Object Reference") (InstigatedBy :type "Controller Object Reference") (DamageCauser :type "Actor Object Reference"))
  ;[1 1 1] Damage control systems (disabled for now)
)

(event `self.ReceiveTick`
  (params (DeltaSeconds :type "Float (single-precision)"))
  (bind _filltime (`self.FillTime`))
  (bind _returnvalue (`PlayerController.GetInputKeyTimeDown` (`GameplayStatics.GetPlayerController` 0) "B"))
  ;[1 1 1] Teleport to Hub System
  (`/Game/Blueprints/UI/WB_BackToHubBtn.UpdateClickProgress` (`self.WB_BackToHabBtn`) (/ _returnvalue _filltime))
  (if (>= _returnvalue _filltime)
    (`/Engine/EditorBlueprintResources/StandardMacros.DoOnce` false :!label _label
      (:`Completed`
        (`self.BackToHub`)))
    (else
      (goto _label :!via `Reset`))))

(event `BackToHub`
  ;[1 1 1] Teleport to Hub System
  (`self.K2_TeleportTo` (-130.0 420.0 590.0)))

(event `EnterInHub`
  (set `/Game/Blueprints/UI/WB_ImplantStore.InHub` true (`self.WB_ImplantStore`))
  (set `Widget.Visibility` "Hidden" (`self.WB_ImplantStore`) :!label _label_2)
  (set `PlayerController.bShowMouseCursor` false (`GameplayStatics.GetPlayerController` 0))
  (`/Game/Blueprints/UI/WB_ImplantStore.CleanUpSelect` (`self.WB_ImplantStore`)))

(event `LogOutHub`
  (set `/Game/Blueprints/UI/WB_ImplantStore.InHub` false (`self.WB_ImplantStore`))
  (goto _label_2))

(fn `UserConstructionScript`)